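; Drivable pirate ship pawn that the player can board and steer.
; A box overlap with BP_Main shows a text prompt and enables Interact, which freezes character movement, blends to the ship camera and possesses the boat.
; Throttle applies force along the right vector, steering adds fixed yaw only under throttle, and Tick pins the character to the Cone's position.
; E hands control back once throttle is zero, using timed delays around the blend.
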(event `InputAxis|Move Forward / Backward`
  (params (AxisValue :type "Float (single-precision)"))
  (bind _output_get (set `self.Up/Down Axis` AxisValue))
  (if (!= _output_get 0.0)
    (set `self.Going Forward` true)
    (`PrimitiveComponent.AddForce` (`self.PirateShip`) (* (* _output_get -2000.0) (`self.GetActorRightVector`)) "None" true)
    (else
      (set `self.Going Forward` false))))

(event `InputAxis|Move Right / Left`
  (params (AxisValue :type "Float (single-precision)"))
  (bind _output_get (set `self.Axis Value` AxisValue))
  (if (!= _output_get 0.0)
    (if (`self.Going Forward`)
      (if (> _output_get 0.0)
        (`SceneComponent.K2_AddLocalRotation` (`self.PirateShip`) (`KismetMathLibrary.MakeRotator` 0.0 0.0 1.25) false false)
        (else
          (`SceneComponent.K2_AddLocalRotation` (`self.PirateShip`) (`KismetMathLibrary.MakeRotator` 0.0 0.0 -1.25) false false))))))

(event `self.ReceiveTick`
  (params (DeltaSeconds :type "Float (single-precision)"))
  (if (`self.Driving`)
    (`self.Handle Player Pos`)))

(event `/Game/Blueprints/World/Object_Interact.Interact`
  (if (`self.Drivable`)
    (if (not (`self.Driving`))
      (set `self.Driving` true)
      (`ActorComponent.Deactivate` (`Character.CharacterMovement` (`self.As BP Main`)))
      (`KismetSystemLibrary.Delay` 0.2)
      (`PlayerController.SetViewTargetWithBlend` (`GameplayStatics.GetPlayerController` 0) (`ActorComponent.GetOwner` (`self.Ship Camera`)) 2.6 "VTBlend_Linear" 0.0 false)
      (`SceneComponent.SetHiddenInGame` (`self.TextRender`) true false)
      (`KismetSystemLibrary.Delay` 2.6)
      (set `self.Can Cancel` true)
      (`Controller.Possess` (`GameplayStatics.GetPlayerController` 0) self))))

(event `Key|E`
  (params (Key :type "Key Structure"))
  (:`Pressed`
    (if (== (`self.Up/Down Axis`) 0.0)
      (if (and (`self.Can Cancel`) (`self.Driving`))
        (set `self.Driving` false)
        (`KismetSystemLibrary.Delay` 0.2)
        (`PlayerController.SetViewTargetWithBlend` (`GameplayStatics.GetPlayerController` 0) (`ActorComponent.GetOwner` (`/Game/ThirdPerson/Blueprints/BP_Main.FollowCamera` (`self.As BP Main`))) 2.6 "VTBlend_Linear" 0.0 false)
        (`SceneComponent.SetHiddenInGame` (`self.TextRender`) false false)
        (`KismetSystemLibrary.Delay` 3.0)
        (`ActorComponent.Activate` (`Character.CharacterMovement` (`self.As BP Main`)) false)
        (set `self.Can Cancel` false)
        (`Controller.Possess` (`GameplayStatics.GetPlayerController` 0) (`self.As BP Main`))))))

(event `self.Box.OnComponentBeginOverlap`
  (params (OverlappedComponent :type "PrimitiveComponent Object Reference") (OtherActor :type "Actor Object Reference") (OtherComp :type "PrimitiveComponent Object Reference") (OtherBodyIndex :type Integer) (bFromSweep :type Boolean) (SweepResult :type "HitResult Structure (by ref)"))
  (bind _asbp_main (cast `/Game/ThirdPerson/Blueprints/BP_Main` OtherActor))
  (set `self.As BP Main` _asbp_main)
  (`SceneComponent.SetHiddenInGame` (`self.TextRender`) false false)
  (set `self.Drivable` true))

(event `self.Box.OnComponentEndOverlap`
  (params (OverlappedComponent :type "PrimitiveComponent Object Reference") (OtherActor :type "Actor Object Reference") (OtherComp :type "PrimitiveComponent Object Reference") (OtherBodyIndex :type Integer))
  (cast `/Game/ThirdPerson/Blueprints/BP_Main` OtherActor)
  (`SceneComponent.SetHiddenInGame` (`self.TextRender`) true false)
  (set `self.Drivable` false)
  (`ActorComponent.Activate` (`Character.CharacterMovement` (`self.As BP Main`)) false))

(fn `Handle Player Pos`
  (bind _output_get (set `self.New Player Pos` (`SceneComponent.K2_GetComponentLocation` (`self.Cone`))))
  (bind (_x _y _z) (`KismetMathLibrary.BreakVector3f` _output_get))
  (`self.K2_SetActorTransform` (`self.As BP Main`) (`KismetMathLibrary.MakeTransform` (`KismetMathLibrary.MakeVector` _x _y _z) (`KismetMathLibrary.MakeRotator` (.roll (`SceneComponent.RelativeRotation` (`self.PirateShip`))) (.pitch (`SceneComponent.RelativeRotation` (`self.PirateShip`))) (+ (.yaw (`SceneComponent.RelativeRotation` (`self.PirateShip`))) (`self.PlayerRotate`)))) false false))

(fn `UserConstructionScript`
  (`SceneComponent.SetHiddenInGame` (`self.TextRender`) true false))
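; Key_BP is a collectible key actor that grants the player's wizard a colored key on overlap.
; When the player pawn enters the sphere collider, the key's mesh material decides whether the Gold, Green or Red key flag is set on Wizard_BP.
; It then plays a pickup sound, calls the wizard's KeyCollected function and destroys itself.
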(event `self.SphereCollider.OnComponentBeginOverlap`
  (params (OverlappedComponent :type "PrimitiveComponent Object Reference") (OtherActor :type "Actor Object Reference") (OtherComp :type "PrimitiveComponent Object Reference") (OtherBodyIndex :type Integer) (bFromSweep :type Boolean) (SweepResult :type "HitResult Structure (by ref)"))
  (bind _returnvalue (`GameplayStatics.GetPlayerPawn` 0))
  (bind _returnvalue_2 (`PrimitiveComponent.GetMaterial` (`self.StaticMesh`) 0))
  (if (== OtherActor _returnvalue)
    (bind _aswizard_bp (cast `/Game/ThirdPerson/Blueprints/Wizard_BP` _returnvalue))
    (if (== _returnvalue_2 "/Game/Kenney_Assets/Platforming/Materials/gold.gold")
      (set `/Game/ThirdPerson/Blueprints/Wizard_BP.Gold Key` true _aswizard_bp))
    (if (== _returnvalue_2 "/Game/Kenney_Assets/Platforming/Materials/greenKey.greenKey")
      (set `/Game/ThirdPerson/Blueprints/Wizard_BP.Green Key` true _aswizard_bp))
    (if (== _returnvalue_2 "/Game/Kenney_Assets/Platforming/Materials/redKey.redKey")
      (set `/Game/ThirdPerson/Blueprints/Wizard_BP.Red Key` true _aswizard_bp))
    (`GameplayStatics.PlaySound2D` "/Game/ItemSounds/WAV/Coins_12.Coins_12" 1.0 1.0 0.0 null null)
    (`/Game/ThirdPerson/Blueprints/Wizard_BP.Key Collected` _aswizard_bp)
    (`self.K2_DestroyActor`)))

(fn `UserConstructionScript`)
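; BP_Sign is a world sign that shows its text when interacted with and hides it when BP_Main leaves its InteractZone.
; While the text is visible, Tick calls a billboard function that yaws SignText from the sign's location toward the player camera.
; Pitch and roll come from a look-at between the actor's location and itself, so the text stays upright.
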(event `/Game/Blueprints/World/Object_Interact.Interact`
  (`SceneComponent.SetHiddenInGame` (`self.Sign Text`) false false))

(event `self.Interact Zone.OnComponentEndOverlap`
  (params (OverlappedComponent :type "PrimitiveComponent Object Reference") (OtherActor :type "Actor Object Reference") (OtherComp :type "PrimitiveComponent Object Reference") (OtherBodyIndex :type Integer))
  (cast `/Game/ThirdPerson/Blueprints/BP_Main` OtherActor)
  (`SceneComponent.SetHiddenInGame` (`self.Sign Text`) true false))

(event `self.ReceiveTick`
  (params (DeltaSeconds :type "Float (single-precision)"))
  ;[1 1 1] Billboard Effect
  (if (not (`SceneComponent.bHiddenInGame` (`self.Sign Text`)))
    (`self.Billboard Effect`)))

(fn `Billboard Effect`
  (bind _returnvalue (`self.K2_GetActorLocation`))
  (`SceneComponent.K2_SetWorldRotation` (`self.Sign Text`) (`KismetMathLibrary.MakeRotator` (.roll (`KismetMathLibrary.FindLookAtRotation` _returnvalue _returnvalue)) (.pitch (`KismetMathLibrary.FindLookAtRotation` _returnvalue _returnvalue)) (.yaw (`KismetMathLibrary.FindLookAtRotation` _returnvalue (`self.K2_GetActorLocation` (`GameplayStatics.GetPlayerCameraManager` 0))))) false false))

(fn `UserConstructionScript`)
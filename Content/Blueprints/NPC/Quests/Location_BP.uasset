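; Location trigger actor that completes a quest when BP_Main enters its box.
; On overlap it loops through BP_Main's active quests and calls QuestComplete where the quest info's actor reference is this actor.
; It then searches all actors of a class and fires EventQuestComplete on those whose quest reference has the same quest name.
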(event `self.Box.OnComponentBeginOverlap`
  (params (OverlappedComponent :type "PrimitiveComponent Object Reference") (OtherActor :type "Actor Object Reference") (OtherComp :type "PrimitiveComponent Object Reference") (OtherBodyIndex :type Integer) (bFromSweep :type Boolean) (SweepResult :type "HitResult Structure (by ref)"))
  (bind (_questinfo_questname _questinfo_actorreference) (break `` (`self.QuestInfo`)))
  (bind _asbp_main (cast `/Game/ThirdPerson/Blueprints/BP_Main` _))
  (for _array_element (`/Game/ThirdPerson/Blueprints/BP_Main.Active Quests` _asbp_main)
    (set `self.Quest Name` (`/Game/Blueprints/NPC/Quests/BP_Quest.QuestName` _array_element))
    (if (== self _questinfo_actorreference)
      (`self.QuestComplete`)
      (bind _outactors (`GameplayStatics.GetAllActorsOfClass` null))
      (for _array_element_2 _outactors
        (bind _questref_questname (break `` (`/Game/Blueprints/NPC/Quests/Location_BP.QuestRef` _array_element_2)))
        (if (`KismetTextLibrary.EqualEqual_TextText` _questinfo_questname _questref_questname)
          (`self.EventQuestComplete` _array_element_2))))))

(fn `UserConstructionScript`)
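; BP_QuestLocationTrigger is a box trigger that completes quests when the player character (BP_Main) reaches its location.
; On overlap it loops through BP_Main's active quests and calls QuestComplete on each if BP_Main's ActorReference is this trigger.
; It then searches all BP_NPC actors and fires EventQuestComplete on those whose QuestActor is this trigger.
; If Destroy is set, the trigger destroys itself after notifying a matching NPC.
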(event `self.Box.OnComponentBeginOverlap`
  (params (OverlappedComponent :type "PrimitiveComponent Object Reference") (OtherActor :type "Actor Object Reference") (OtherComp :type "PrimitiveComponent Object Reference") (OtherBodyIndex :type Integer) (bFromSweep :type Boolean) (SweepResult :type "HitResult Structure (by ref)"))
  (bind _asbp_main (cast `/Game/ThirdPerson/Blueprints/BP_Main` OtherActor))
  (set `self.As BP Main` _asbp_main)
  (for _array_element (`/Game/ThirdPerson/Blueprints/BP_Main.Active Quests` _asbp_main)
    (set `self.Quest` _array_element)
    (set `self.Quest Name` (`/Game/Blueprints/NPC/Quests/BP_Quest.QuestName` _array_element))
    (if (== self (`/Game/ThirdPerson/Blueprints/BP_Main.Actor Reference` _asbp_main))
      (`/Game/ThirdPerson/Blueprints/BP_Main.QuestComplete` (`self.As BP Main`) (`self.Quest`))
      (bind _outactors (`GameplayStatics.GetAllActorsOfClass` "/Game/Blueprints/NPC/BP_NPC.BP_NPC_C"))
      (for _array_element_2 _outactors
        (if (== (`/Game/Blueprints/NPC/BP_NPC.Quest Actor` _array_element_2) self)
          (`/Game/Blueprints/NPC/BP_NPC.EventQuestComplete` _array_element_2)
          (if (`self.Destroy?`)
            (`self.K2_DestroyActor`)))))))

(fn `UserConstructionScript`)
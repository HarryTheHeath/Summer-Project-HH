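; NPC actor that shows a prompt when BP_Main enters its interact zone and runs a dialogue with the player.
; TriggerDialogue locks movement, switches to UI input and the NPC's camera, teleports the player to the Cone marker, then opens the NPC_Dialogue widget with ConversationInfo.
; EndDialogue blends back to the follow camera and restores control.
; The construction script places camera and marker from per-instance variables.
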(event `self.Interact Zone.OnComponentBeginOverlap`
  (params (OverlappedComponent :type "PrimitiveComponent Object Reference") (OtherActor :type "Actor Object Reference") (OtherComp :type "PrimitiveComponent Object Reference") (OtherBodyIndex :type Integer) (bFromSweep :type Boolean) (SweepResult :type "HitResult Structure (by ref)"))
  ;[1 1 1] Hide Prompt Text
  (bind _asbp_main (cast `/Game/ThirdPerson/Blueprints/BP_Main` OtherActor))
  (set `self.As BP Main` _asbp_main)
  (`SceneComponent.SetHiddenInGame` (`self.Dialogue`) false false)
  (`SceneComponent.SetHiddenInGame` (`self.Background`) false false))

(event `self.Interact Zone.OnComponentEndOverlap`
  (params (OverlappedComponent :type "PrimitiveComponent Object Reference") (OtherActor :type "Actor Object Reference") (OtherComp :type "PrimitiveComponent Object Reference") (OtherBodyIndex :type Integer))
  ;[1 1 1] Hide Prompt Text
  (bind _asbp_main (cast `/Game/ThirdPerson/Blueprints/BP_Main` OtherActor))
  (set `self.As BP Main` _asbp_main)
  (`SceneComponent.SetHiddenInGame` (`self.Dialogue`) true false :!label _label)
  (`SceneComponent.SetHiddenInGame` (`self.Background`) true false))

(event `self.ReceiveBeginPlay`
  ;[1 1 1] Create Dialogue Widget
  (bind _returnvalue (`|CreateWidget` "/Game/Blueprints/NPC/NPC_Dialogue.NPC_Dialogue_C"))
  (bind _output_get (set `self.NPCChat` _returnvalue))
  (set `/Game/Blueprints/NPC/NPC_Dialogue.NPC_Ref` self _output_get)
  (`Widget.SetVisibility` (`self.NPCChat`) "Hidden")
  (set `self.PControl` (`GameplayStatics.GetPlayerController` 0))
  (goto _label))

(event `/Game/Blueprints/NPC/NPC_Interact.Trigger Dialogue`
  ;[1 1 1] Trigger Dialogue (Set-Up)
  (`self.Transition`)
  (`KismetSystemLibrary.Delay` 0.4)
  (`self.Begin Dialogue`)
  (goto _label))

(event `Transition`
  (bind (_returnvalue_x _returnvalue_y) (`KismetMathLibrary.BreakVector` (`SceneComponent.K2_GetComponentLocation` (`self.Cone`))))
  (bind (_returnvalue_roll _returnvalue_pitch _returnvalue_yaw) (`KismetMathLibrary.BreakRotator` (`SceneComponent.K2_GetComponentRotation` (`self.Mesh`))))
  (bind _rootcomponent (`Actor.RootComponent` (`self.As BP Main`)))
  (bind (_returnvalue_roll_2 _returnvalue_pitch_2) (`KismetMathLibrary.BreakRotator` (`SceneComponent.K2_GetComponentRotation` _rootcomponent)))
  (bind (_returnvalue_x_2 _returnvalue_y_2 _returnvalue_z) (`KismetMathLibrary.BreakVector` (`SceneComponent.K2_GetComponentLocation` _rootcomponent)))
  ;[1 1 1] Start Transition + Disable Movement
  (set `PlayerController.bShowMouseCursor` true (`self.PControl`))
  (`ActorComponent.Deactivate` (`Character.CharacterMovement` (`self.As BP Main`)))
  (`WidgetBlueprintLibrary.SetInputMode_UIOnlyEx` (`self.PControl`) null)
  ;[1 1 1] Camera Teleport
  (`KismetSystemLibrary.Delay` 0.2)
  (`PlayerController.SetViewTargetWithBlend` (`self.PControl`) (`ActorComponent.GetOwner` (`self.Camera`)) 0.0 "VTBlend_Linear" 0.0 false)
  (`SceneComponent.K2_SetWorldTransform` _rootcomponent (`KismetMathLibrary.MakeTransform` (`KismetMathLibrary.MakeVector` _returnvalue_x _returnvalue_y _returnvalue_z) (`KismetMathLibrary.MakeRotator` _returnvalue_roll_2 _returnvalue_pitch_2 (+ _returnvalue_yaw -90.0))) false false))

(event `Begin Dialogue`
  (bind _npcchat (`self.NPCChat`))
  ;[1 1 1] Begin Dialogue
  (`/Game/Blueprints/NPC/NPC_Dialogue.Begin` _npcchat (`self.Conversation Info`))
  (`UserWidget.AddToViewport` _npcchat 0)
  (`Widget.SetVisibility` (`self.NPCChat`) "Visible"))

(event `End Dialogue`
  (bind _pcontrol (`self.PControl`))
  ;[1 1 1] End Dialogue
  (`Widget.RemoveFromParent` (`self.NPCChat`))
  (`PlayerController.SetViewTargetWithBlend` (`self.PControl`) (`ActorComponent.GetOwner` (`/Game/ThirdPerson/Blueprints/BP_Main.FollowCamera` (`self.As BP Main`))) 1.3 "VTBlend_Linear" 0.0 false)
  (`KismetSystemLibrary.Delay` 1.3)
  (`WidgetBlueprintLibrary.SetInputMode_GameOnly` _pcontrol)
  (set `PlayerController.bShowMouseCursor` false _pcontrol)
  (`ActorComponent.Activate` (`Character.CharacterMovement` (`self.As BP Main`)) false))

(fn `Evaluate Player Scale`
  (set `self.Player Scale` (`SceneComponent.K2_GetComponentScale` (`Character.Mesh` (`self.As BP Main`)))))

(fn `UserConstructionScript`
  (`SceneComponent.K2_SetRelativeTransform` (`self.Camera`) (`self.CamPos`) false false)
  (`SceneComponent.K2_SetRelativeLocation` (`self.Cone`) (`self.PlayerPos`) false false)
  (`SceneComponent.K2_SetRelativeRotation` (`self.Cone`) (`self.Player Rotate`) false false))